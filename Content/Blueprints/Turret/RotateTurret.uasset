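; RotateTurret is a behavior tree task that aims a turret's gun at a target location stored on the blackboard.
; On execute it casts the controlled pawn to Turret and computes a look-at rotation from the GunArrow component to that location.
; It instantly sets the arrow's world pitch and yaw with zero roll, then finishes successfully, or fails when the cast fails.
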(event EventReceiveExecuteAI
  (params (OwnerController :type AI%20Controller%20Object%20Reference) (ControlledPawn :type Pawn%20Object%20Reference))
  ;[1 1 1] setta para onde a arma da torre deve girar
  (bind _asturret (Utilities|Casting|CastToTurret ControlledPawn)
    (:then
      ;[1 1 1] gira a arma da torre
      (Transformation|SetWorldRotation (Variables|/Game/Blueprints/Turret/Turret.Turret_C|GetGunArrow _asturret) (Math|Rotator|MakeRotator 0.0 (.Pitch (Math|Rotator|BreakRotator (Math|Rotator|FindLookatRotation (Transformation|GetWorldLocation (Variables|/Game/Blueprints/Turret/Turret.Turret_C|GetGunArrow _asturret)) (Class|BTFunctionLibrary|GetBlackboardValueasVector (Variables|Default|GetPLocation))))) (.Yaw (Math|Rotator|BreakRotator (Math|Rotator|FindLookatRotation (Transformation|GetWorldLocation (Variables|/Game/Blueprints/Turret/Turret.Turret_C|GetGunArrow _asturret)) (Class|BTFunctionLibrary|GetBlackboardValueasVector (Variables|Default|GetPLocation)))))) false false)
      (AI|BehaviorTree|FinishExecute true))
    (:CastFailed
      (AI|BehaviorTree|FinishExecute false))))