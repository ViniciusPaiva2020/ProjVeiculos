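; ShootTurret is a behavior tree task that makes an AI-controlled Turret fire a TurretProjectile from its FireArrow transform.
; A shot sets the CD cooldown flag, and later executions add frame delta time to Timer until TotalCD clears it, printing a debug "fire".
; The task finishes immediately on each execution, so the cooldown relies on repeated re-execution, and it fails only when an attempted shot's Turret cast fails.
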(event EventReceiveExecuteAI
  (params (OwnerController :type AI%20Controller%20Object%20Reference) (ControlledPawn :type Pawn%20Object%20Reference))
  (if (Variables|Default|GetCD)
    (bind _output_get (Variables|Default|Settimer (+ (Variables|Default|Gettimer) (Utilities|Time|GetWorldDeltaSeconds))))
    (if (>= _output_get (Variables|Default|GettotalCD))
      (Variables|Default|SetCD false)
      (Variables|Default|Settimer 0.0)
      (Development|PrintString "fire"))
    (AI|BehaviorTree|FinishExecute true :!label _label)
    (else
      (bind _asturret (Utilities|Casting|CastToTurret ControlledPawn)
        (:then
          (Game|SpawnActorfromClass "/Game/Blueprints/Turret/TurretProjectile.TurretProjectile_C" (Transformation|GetWorldTransform (Variables|/Game/Blueprints/Turret/Turret.Turret_C|GetFireArrow _asturret)) "Undefined" 0 0)
          (Variables|Default|SetCD true)
          (goto _label))
        (:CastFailed
          (AI|BehaviorTree|FinishExecute false))))))