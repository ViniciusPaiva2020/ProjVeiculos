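; AI controller for the turret that detects the player and feeds the turret's behavior tree.
; It runs BT_Turret on BeginPlay, and perception updates set PlayerSpotted in the blackboard when an actor tagged Player is sensed, storing that actor.
; While the player is spotted, Tick writes the stored actor's root component world location to the PlayerLocation key.
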(event OnTargetPerceptionUpdated(AIPerception)
  (params (Actor :type Actor%20Object%20Reference) (Stimulus :type AI%20Stimulus%20Structure))
  ;[1 1 1] checa se o player for visto
  ;;[1 1 1] setta variáveis usadas pela AI
  (bind _output_get (Variables|Default|SetSpotted (and (Actor|ActorHasTag Actor "Player") (.bSuccessfullySensed (Utilities|Struct|BreakAIStimulus Stimulus)))))
  (AI|Components|Blackboard|SetValueasBool (AI|GetBlackboard 0) (Utilities|Name|MakeLiteralName "PlayerSpotted") _output_get)
  (if _output_get
    (bind _output_get_2 (Variables|Default|SetPlayer Actor))
    (Development|PrintString (Utilities|GetDisplayName _output_get_2))))

(event EventBeginPlay
  ;[1 1 1] inicia a AI
  (AI|RunBehaviorTree "/Game/Blueprints/Turret/BT_Turret.BT_Turret"))

(event EventTick
  (params (DeltaSeconds :type Float%20%28single-precision%29))
  ;[1 1 1] pega a localização do objeto do player, incluindo veículos
  (if (Variables|Default|GetSpotted)
    (AI|Components|Blackboard|SetValueasVector (AI|GetBlackboard 0) (Utilities|Name|MakeLiteralName "PlayerLocation") (Transformation|GetWorldLocation (Variables|/Script/Engine.Actor|GetRootComponent (Variables|Default|GetPlayer))))))

(fn ConstructionScript)